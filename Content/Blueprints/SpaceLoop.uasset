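; SpaceLoop is an endless track generator that lays biome-themed pieces along the X axis and destroys those the player pawn has left behind.
; PickTrack shuffles presets and reads class defaults to queue a Start, then Mid pieces, with a random End and biome switch after a minimum length.
; Tick calls SpawnTrack when the track runs short, spawning queued pieces at an offset advanced by their dimensions, then picking another.
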(event EventBeginPlay
  ;[1 1 1] Spawn track pieces
  (CallFunction|ListBiomes)
  (Variables|Default|SetCurrentBiome (Variables|Default|GetStartBiome))
  (while (> (Variables|Default|GetTrackLength) (Utilities|Array|Length (Variables|Default|GetToSpawn)))
    (CallFunction|PickTrack)))

(event EventTick
  (params (DeltaSeconds :type Float%20%28single-precision%29))
  (bind _trackpieces (Variables|Default|GetTrackPieces))
  (if (< (Utilities|Array|Length _trackpieces) (Variables|Default|GetTrackLength))
    (CallFunction|SpawnTrack))
  (bind _array_element (Utilities|Array|ForEachLoopwithBreak _trackpieces)
    (:LoopBody
      (if (> (.X (Math|Vector|BreakVector (Transformation|GetActorLocation (Game|Player|GetPlayerPawn 0)))) (+ (+ (.X (Math|Vector|BreakVector (Transformation|GetActorLocation _array_element))) (/ (.X (Math|Vector|BreakVector (Variables|/Game/Blueprints/Track/Track.Track_C|GetDimensions _array_element))) 2.0)) 5e+03))
        (Actor|DestroyActor _array_element)
        (Utilities|Array|RemoveItem _trackpieces _array_element)))))

(fn ConstructionScript)

(fn SpawnTrack
  (bind _tospawn (Variables|Default|GetToSpawn))
  (bind (_array_element _array_index) (Utilities|Array|ForEachLoopwithBreak _tospawn)
    (:LoopBody
      (bind _returnvalue (Game|SpawnActorfromClass _array_element (Math|Conversions|ToTransform(Vector) (Variables|Default|GetTrackPlacementOffset)) "Undefined" 0 0))
      (Utilities|Array|Add (Variables|Default|GetTrackPieces) _returnvalue)
      (Variables|Default|SetTrackPlacementOffset (Math|Vector|MakeVector (.X (Math|Vector|BreakVector (+ (Variables|Default|GetTrackPlacementOffset) (.Dimensions (Utilities|GetClassDefaults _array_element))))) 0.0 0.0))
      (Utilities|Array|RemoveIndex _tospawn _array_index))
    (:Completed
      (CallFunction|PickTrack))))

(fn PickTrack
  (bind _returnvalue (Math|Random|RandomInteger 100))
  (bind _trackpresets (Variables|Default|GetTrackPresets))
  (bind _tospawn (Variables|Default|GetToSpawn))
  (bind _biometypes (Variables|Default|GetBiomeTypes))
  (Utilities|Array|Shuffle _trackpresets)
  (bind _array_element (Utilities|Array|ForEachLoopwithBreak _trackpresets)
    (:LoopBody
      (if (not (LocalVariables|GetFoundTrack))
        (if (== (.Biome (Utilities|GetClassDefaults _array_element)) (Variables|Default|GetCurrentBiome))
          (if (<= (Variables|Default|GetCurrentBiomeLength) 0)
            (if (Utilities|Name|Equal(Name) (.SectionType (Utilities|GetClassDefaults _array_element)) "Start")
              (Utilities|Array|Add _tospawn _array_element)
              (Math|Integer|IncrementInt (Variables|Default|GetCurrentBiomeLength) :!label _label
                (:%20%20
                  (LocalVariables|SetFoundTrack true))))
            (elif (Utilities|Name|Equal(Name) (.SectionType (Utilities|GetClassDefaults _array_element)) "Mid")
              (Utilities|Array|Add _tospawn _array_element)
              (goto _label))))))
    (:Completed
      (if (LocalVariables|GetFoundTrack)
        (if (>= (Variables|Default|GetCurrentBiomeLength) (Variables|Default|GetMinBiomeLength))
          (if (<= _returnvalue (/ _returnvalue 2))
            (Utilities|Array|Shuffle _trackpresets)
            (bind _array_element_2 (Utilities|Array|ForEachLoopwithBreak _trackpresets)
              (:LoopBody
                (if (not (LocalVariables|GetFoundEnd))
                  (if (and (== (Variables|Default|GetCurrentBiome) (.Biome (Utilities|GetClassDefaults _array_element_2))) (Utilities|Name|Equal(Name) (.SectionType (Utilities|GetClassDefaults _array_element_2)) "End"))
                    (Utilities|Array|Add (Variables|Default|GetToSpawn) _array_element_2)
                    (Utilities|Array|Shuffle _biometypes)
                    (bind _array_element_3 (Utilities|Array|ForEachLoopwithBreak _biometypes)
                      (:LoopBody
                        (if (not (LocalVariables|GetFoundBiome))
                          (if (not (== _array_element_3 (Variables|Default|GetCurrentBiome)))
                            (Variables|Default|SetCurrentBiome _array_element_3)
                            (Variables|Default|SetCurrentBiomeLength 0)
                            (LocalVariables|SetFoundBiome true))))
                      (:Completed
                        (LocalVariables|SetFoundEnd true)
                        (if (not (LocalVariables|GetFoundBiome))
                          (Development|PrintString "The generator was unable to find a new biome to use.")))))))
              (:Completed
                (if (not (LocalVariables|GetFoundEnd))
                  (Development|PrintString "The generator was unable to find an endpiece to use."))))))
        (else
          (Development|PrintString "The generator was unable to find a track piece to use."))))))

(fn ListBiomes
  (bind _biometypes (Variables|Default|GetBiomeTypes))
  (bind _array_element (Utilities|Array|ForEachLoopwithBreak (Variables|Default|GetTrackPresets))
    (:LoopBody
      (if (not (Utilities|Array|ContainsItem _biometypes (.Biome (Utilities|GetClassDefaults _array_element))))
        (Utilities|Array|Add _biometypes (.Biome (Utilities|GetClassDefaults _array_element)))))))